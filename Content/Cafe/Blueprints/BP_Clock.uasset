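; BP_Clock is a cafe wall clock prop whose two hands show progress through the game day.
; On BeginPlay it caches BP_CafeGameMode, then each Tick reads elapsed time as a fraction of day length.
; That fraction lerps each hand's relative pitch, spinning one through six full turns while the other sweeps half a turn.
; When it is not day, both hands are set to zero rotation.
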(event `self.ReceiveBeginPlay`
  (bind _asbp_cafe_game_mode (cast `/Game/Cafe/Blueprints/BP_CafeGameMode` (`GameplayStatics.GetGameMode`)))
  (set `self.As BP Cafe Game Mode` _asbp_cafe_game_mode))

(event `self.ReceiveTick`
  (params (DeltaSeconds :type "Float (single-precision)"))
  (bind _as_bp_cafe_game_mode (`self.As BP Cafe Game Mode`))
  (bind _returnvalue (/ (`CafeGameModeBase.GetTimeElapsed` _as_bp_cafe_game_mode) (`/Game/Cafe/Blueprints/BP_CafeGameMode.DayLength` _as_bp_cafe_game_mode)))
  (if (`/Game/Cafe/Blueprints/BP_CafeGameMode.IsDay` _as_bp_cafe_game_mode)
    (`SceneComponent.K2_SetRelativeRotation` (`self.SM_Clock_Corkboard_Catsign_Bighand1`) (`KismetMathLibrary.MakeRotator` 0.0 (`KismetMathLibrary.Lerp` 0.0 2160.0 _returnvalue)) false false)
    (`SceneComponent.K2_SetRelativeRotation` (`self.SM_Clock_Corkboard_Catsign_Bighand2`) (`KismetMathLibrary.MakeRotator` 0.0 (`KismetMathLibrary.Lerp` 180.0 360.0 _returnvalue)) false false)
    (else
      (`SceneComponent.K2_SetRelativeRotation` :`self` (`self.SM_Clock_Corkboard_Catsign_Bighand1`))
      (`SceneComponent.K2_SetRelativeRotation` :`self` (`self.SM_Clock_Corkboard_Catsign_Bighand2`)))))

(fn `UserConstructionScript`)