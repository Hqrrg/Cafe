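; BP_MilkStation is the milk station in the cafe game, where the barista works with milk ingredients for the current order.
; On interact it runs the parent logic, then, if the barista holds a valid order, opens a WBP_Station widget fed with its ingredient array and milk-specific artwork.
; It plays a glass bottle opening sound when an ingredient is made and removes the widget on exit.
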(event `self.OnIngredientMade`
  (params (Ingredient :type "EIngredient Enum" :default "Water"))
  (`GameplayStatics.PlaySound2D` "/Game/Cafe/Audio/SFX/Other/glass-bottle-open-86299-_AudioTrimmer_com_.glass-bottle-open-86299-_AudioTrimmer_com_" 1.0 1.0 0.0 null null))

(event `self.Interact`
  (`parent.Interact`)
  (`/Engine/EditorBlueprintResources/StandardMacros.IsValid` (`BaristaCharacter.GetCurrentOrder` (`self.GetBaristaRef`))
    (:`Is Valid`
      (bind _returnvalue (`|CreateWidget` "/Game/Cafe/Blueprints/WBP_Station.WBP_Station_C" (`GameplayStatics.GetPlayerController` 0) (`self.GetIngredientArray`) self "/Game/Cafe/Textures/UI/T_MilkStationBackground.T_MilkStationBackground" "/Game/Cafe/Textures/UI/T_Equals_Milk.T_Equals_Milk"))
      (bind _output_get (set `self.WBPStation` _returnvalue))
      (`UserWidget.AddToViewport` _output_get 0))))

(event `self.OnExit`
  (`Widget.RemoveFromParent` (`self.WBPStation`)))

(fn `UserConstructionScript`)