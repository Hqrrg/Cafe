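; BP_Barista is the cafe game's barista Blueprint, which manages the player's HUD and end-of-day shop screen.
; On BeginPlay it creates the HUD with balance, profit quota and day from CafeGameModeBase and binds to that game mode's OnEndDay.
; When the day ends, it swaps the HUD for the shop widget.
; Pressing the 1 key calls the game mode's EndDay directly with a false argument.
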(event `self.ReceiveBeginPlay`
  (`parent.ReceiveBeginPlay`)
  (bind _ascafe_game_mode_base (cast `CafeGameModeBase` (`GameplayStatics.GetGameMode`)))
  (add `CafeGameModeBase.OnEndDay` _ascafe_game_mode_base (delegate `EndDay`))
  (bind _returnvalue (`|CreateWidget` "/Game/Cafe/Blueprints/WBP_HUD.WBP_HUD_C" (`GameplayStatics.GetPlayerController` 0) (`CafeGameModeBase.GetBalance` _ascafe_game_mode_base) (`CafeGameModeBase.GetQuota` _ascafe_game_mode_base) (`CafeGameModeBase.GetDay` _ascafe_game_mode_base)))
  (bind _output_get (set `self.HUDWidget` _returnvalue))
  (`UserWidget.AddToViewport` _output_get 0))

(event `EndDay`
  (`Widget.RemoveFromParent` (`self.HUDWidget`))
  (bind _returnvalue (`|CreateWidget` "/Game/Cafe/Blueprints/WBP_Shop.WBP_Shop_C" (`GameplayStatics.GetPlayerController` 0)))
  (`UserWidget.AddToViewport` _returnvalue 0))

(event `Key|One`
  (params (Key :type "Key Structure"))
  (:`Pressed`
    (bind _ascafe_game_mode_base (cast `CafeGameModeBase` (`GameplayStatics.GetGameMode`)))
    (`CafeGameModeBase.EndDay` _ascafe_game_mode_base false)))

(fn `UserConstructionScript`)